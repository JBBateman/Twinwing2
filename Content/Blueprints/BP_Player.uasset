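; Player character for an on-rails flying shooter, pushed constantly along world +Y while input moves it sideways and vertically within clamped camera angles.
; Aim input moves the crosshair widget and a Target component, and shooting line-traces from Gun to Target to destroy enemies or open loot boxes.
; Events update health, multiplied score and their HUD widgets, plus a damage multiplier that shooting ignores.
; It also handles pause, restart and quit.
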(event `self.ReceiveBeginPlay`
  (bind _returnvalue (`GameplayStatics.GetPlayerCameraManager` 0))
  (bind _returnvalue_2 (`GameplayStatics.GetPlayerController` 0))
  ;[1 1 1] Start
  (`|ExecutionSequence`
    (:`then_0`
      (bind _asplayer_controller (cast `PlayerController` (`self.GetController`)))
      (bind _returnvalue_3 (pcsubsystem `EnhancedInputLocalPlayerSubsystem` _asplayer_controller))
      (`/Engine/EditorBlueprintResources/StandardMacros.IsValid` _returnvalue_3
        (:`Is Valid`
          (`EnhancedInputSubsystemInterface.AddMappingContext` _returnvalue_3 "/Game/Input/IMC_PlayerInput.IMC_PlayerInput" 0 (struct))
          (`CharacterMovementComponent.SetMovementMode` (`self.CharacterMovement`) "MOVE_Flying" 0)
          (set `PlayerCameraManager.ViewPitchMax` 15.0 _returnvalue)
          (set `PlayerCameraManager.ViewPitchMin` -45.0 _returnvalue)
          (set `PlayerCameraManager.ViewYawMax` 225.0 _returnvalue)
          (set `PlayerCameraManager.ViewYawMin` 135.0 _returnvalue)
          ;[1 1 1] crosshair widget
          (bind _returnvalue_4 (`|CreateWidget` "/Game/UI/BP_Crosshair.BP_Crosshair_C" _returnvalue_2))
          (`UserWidget.AddToViewport` _returnvalue_4 0)
          (set `self.CrosshairRef` _returnvalue_4)
          ;[1 1 1] Score widget
          (bind _returnvalue_5 (`|CreateWidget` "/Game/UI/BP_ScoreText.BP_ScoreText_C" _returnvalue_2))
          (`UserWidget.AddToViewport` _returnvalue_5 0)
          (set `self.ScoreWidgetRef` _returnvalue_5)
          (set `self.scoreMultiplier` 1.0))))
    (:`then_1`
      ;[1 1 1] healthbar widget
      (bind _returnvalue_6 (`|CreateWidget` "/Game/UI/HealthbarWidget.HealthbarWidget_C"))
      (bind _output_get (set `self.HealthWidget REF` _returnvalue_6))
      (set `/Game/UI/HealthbarWidget.Max Health` (`self.Max Health`) _output_get)
      (set `/Game/UI/HealthbarWidget.Health` (`self.Health`) _output_get)
      (`UserWidget.AddToViewport` _returnvalue_6 0))))

(event `EnhancedInput|/Game/Input/IA_Pause`
  (params (ActionValue :type Boolean) (ElapsedSeconds :type "Float (double-precision)") (TriggeredSeconds :type "Float (double-precision)") (InputAction :type "InputAction Object Reference" :default "/Game/Input/IA_Pause.IA_Pause"))
  ;[1 1 1] Pause
  (:`Started`
    (if (`self.isPaused`)
      (set `self.isPaused` false)
      (`GameplayStatics.SetGamePaused` false)
      (else
        (set `self.isPaused` true)
        (`GameplayStatics.SetGamePaused` true)))))

(event `EnhancedInput|/Game/Input/IA_Restart`
  (params (ActionValue :type Boolean) (ElapsedSeconds :type "Float (double-precision)") (TriggeredSeconds :type "Float (double-precision)") (InputAction :type "InputAction Object Reference" :default "/Game/Input/IA_Restart.IA_Restart"))
  ;[1 1 1] Restart Game
  (:`Started`
    (bind _asgame_mode (cast `GameMode` (`GameplayStatics.GetGameMode`)))
    (`GameMode.RestartGame` _asgame_mode)))

(event `EnhancedInput|/Game/Input/IA_Fly`
  (params (ActionValue :type "Vector2D Structure") (ElapsedSeconds :type "Float (double-precision)") (TriggeredSeconds :type "Float (double-precision)") (InputAction :type "InputAction Object Reference" :default "/Game/Input/IA_Fly.IA_Fly"))
  (bind (_returnvalue_roll _returnvalue_pitch _returnvalue_yaw) (`KismetMathLibrary.BreakRotator` (`self.GetControlRotation`)))
  ;[1 1 1] Move side to side action
  (:`Triggered`
    (`self.AddMovementInput` (`KismetMathLibrary.GetRightVector` (`KismetMathLibrary.MakeRotator` _returnvalue_roll 0.0 _returnvalue_yaw)) (* ActionValue_X (`self.MovementSpeed`)))
    ;[1 1 1] move up and down action
    (`self.AddMovementInput` (`self.GetActorUpVector` (`self.GetController`)) (* ActionValue_Y (`self.MovementSpeed`)))))

(event `TakeDamage`
  (params (Dmg :type "Float (double-precision)"))
  (bind _returnvalue (- (`self.Health`) Dmg))
  ;[1 1 1] Damage taking
  (bind _output_get (set `self.Health` _returnvalue))
  (set `/Game/UI/HealthbarWidget.Health` _output_get (`self.HealthWidget REF`))
  ;[1 1 1] Death
  (if (<= _returnvalue 0.0)
    (`self.K2_DestroyActor`)))

(event `IncreaseScore`
  (params (points :type "Float (double-precision)"))
  ;[1 1 1] increase and update score
  (bind _output_get (set `self.score` (+ (`self.score`) (* points (`self.scoreMultiplier`)))))
  (`/Game/UI/BP_ScoreText.UpdateScoreText` (`self.ScoreWidgetRef`) (`KismetMathLibrary.Round` _output_get)))

(event `EnhancedInput|/Game/Input/IA_Quit`
  (params (ActionValue :type Boolean) (ElapsedSeconds :type "Float (double-precision)") (TriggeredSeconds :type "Float (double-precision)") (InputAction :type "InputAction Object Reference" :default "/Game/Input/IA_Quit.IA_Quit"))
  ;[1 1 1] Quit
  (:`Started`
    (`KismetSystemLibrary.QuitGame` null "Quit")))

(event `AddHealth`
  (params (HealthAddition :type "Float (double-precision)"))
  ;[1 1 1] AddHealth
  (bind _output_get (set `self.Health` (`KismetMathLibrary.FClamp` (+ (`self.Health`) HealthAddition) 0.0 (`self.Max Health`))))
  (set `/Game/UI/HealthbarWidget.Health` _output_get (`self.HealthWidget REF`)))

(event `IncreaseScoreMultiplier`
  (params (Input :type "Float (double-precision)"))
  ;[1 1 1] increase score multiplier
  (set `self.scoreMultiplier` (+ Input (`self.scoreMultiplier`))))

(event `AddDamageMultiplier`
  (params (DmgAddition :type "Float (double-precision)"))
  ;[1 1 1] Add to Damage Multiplier
  (bind _output_get (set `self.DmgMultiplier` (+ DmgAddition (`self.DmgMultiplier`))))
  (`KismetSystemLibrary.PrintString` (`KismetStringLibrary.Conv_DoubleToString` _output_get)))

(event `self.ReceiveTick`
  (params (DeltaSeconds :type "Float (single-precision)"))
  ;[1 1 1] Fly Forward Distance
  (`self.AddMovementInput` (-0.0 5.0 0.0)))

(event `EnhancedInput|/Game/Input/IA_Aim`
  (params (ActionValue :type "Vector2D Structure") (ElapsedSeconds :type "Float (double-precision)") (TriggeredSeconds :type "Float (double-precision)") (InputAction :type "InputAction Object Reference" :default "/Game/Input/IA_Aim.IA_Aim"))
  ;[1 1 1] Aim
  (:`Triggered`
    (`/Game/UI/BP_Crosshair.MoveCrosshair` (`self.CrosshairRef`) ActionValue)
    (`self.SetTarget` ActionValue)))

(event `EnhancedInput|/Game/Input/IA_Shoot`
  (params (ActionValue :type Boolean) (ElapsedSeconds :type "Float (double-precision)") (TriggeredSeconds :type "Float (double-precision)") (InputAction :type "InputAction Object Reference" :default "/Game/Input/IA_Shoot.IA_Shoot"))
  ;[1 1 1] shooting
  (:`Started`
    (bind (_outhit _returnvalue) (`KismetSystemLibrary.LineTraceSingle` :`Start` (`SceneComponent.K2_GetComponentLocation` (`self.Gun`)) :`End` (`SceneComponent.K2_GetComponentLocation` (`self.Target`)) :`TraceChannel` "TraceTypeQuery1" :`bTraceComplex` true :`DrawDebugType` "Persistent"))
    (if _returnvalue
      (bind (_bblockinghit _binitialoverlap _time _distance _location _impactpoint _normal _impactnormal _physmat _hitactor) (`GameplayStatics.BreakHitResult` _outhit))
      (bind _asbp_enemy_1 (cast `/Game/Blueprints/Enemies/BP_Enemy1` _hitactor)
        (:`then`
          (`/Game/Blueprints/Enemies/BP_Enemy1.DestroyEnemy` _asbp_enemy_1))
        (:`CastFailed`
          (bind _asbp_loot_box (cast `/Game/Blueprints/LootBoxBlueprints/BP_LootBox` _hitactor)
            (:`then`
              (`/Game/Blueprints/LootBoxBlueprints/BP_LootBox.LootDropper` _asbp_loot_box))
            (:`CastFailed`
              _))
          (`KismetSystemLibrary.PrintString` "No HIt" :!label _label)))
      (else
        (goto _label)))))

(fn `SetTarget`
  (params (InputVector :type "Vector2D Structure"))
  (bind (_x _y) (`KismetMathLibrary.BreakVector2D` InputVector))
  (bind _target (`self.Target`))
  (bind _returnvalue (* _x 10.5))
  (bind (_relativelocation_x _relativelocation_y _relativelocation_z) (`KismetMathLibrary.BreakVector` (`SceneComponent.RelativeLocation` _target)))
  (`SceneComponent.K2_SetRelativeLocationAndRotation` :`self` _target :`NewLocation` (`KismetMathLibrary.MakeVector` (+ (`KismetMathLibrary.FClamp` _relativelocation_x -180.0 1780.0) _returnvalue) (+ (`KismetMathLibrary.FClamp` _relativelocation_y -1780.0 180.0) _returnvalue) (+ (* _y -15.0) (`KismetMathLibrary.FClamp` _relativelocation_z -750.0 827.0)))))

(fn `UserConstructionScript`)
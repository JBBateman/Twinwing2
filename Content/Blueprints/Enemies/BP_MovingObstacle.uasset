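; BP_MovingObstacle is an enemy obstacle that moves through the level and destroys any player it touches.
; StartMovement stores the given speed, which Tick adds to the actor location through MakeNewLocation to teleport-free, unswept reposition it.
; The step ignores delta time, so movement depends on frame rate.
; A BoxCollision overlap destroys actors tagged "Player" directly, with no damage step.
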(event `StartMovement`
  (params (MovementSpd :type "Vector Structure"))
  ;[1 1 1] Start Movement
  (set `self.Speed` MovementSpd))

(event `self.ReceiveTick`
  (params (DeltaSeconds :type "Float (single-precision)"))
  (bind _returnvalue_location (`KismetMathLibrary.BreakTransform` (`KismetMathLibrary.MakeTransform` (+ (`self.Speed`) (`self.K2_GetActorLocation`)))))
  ;[1 1 1] Move Obstacle
  (`self.K2_SetActorLocation` _returnvalue_location))

(event `self.BoxCollision.OnComponentBeginOverlap`
  (params (OverlappedComponent :type "PrimitiveComponent Object Reference") (OtherActor :type "Actor Object Reference") (OtherComp :type "PrimitiveComponent Object Reference") (OtherBodyIndex :type Integer) (bFromSweep :type Boolean) (SweepResult :type "HitResult Structure (by ref)"))
  ;[1 1 1] Destroy Player
  (if (`self.ActorHasTag` OtherActor "Player")
    (`self.K2_DestroyActor` OtherActor)))

(fn `UserConstructionScript`)
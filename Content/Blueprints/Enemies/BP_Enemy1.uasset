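; BP_Enemy1 is an enemy that chases the player and deals damage on contact.
; ProjectileMovement homes on the player's capsule, set at BeginPlay.
; Box overlap damages the player without destroying the enemy, ignores other BP_Enemy1 actors and destroys the enemy on anything else.
; TakeDamage only lowers Health because the zero-health check is disconnected, leaving DestroyEnemy as an explicit way to remove it.
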(event `self.ReceiveBeginPlay`
  ;[1 1 1] Add player target
  (set `ProjectileMovementComponent.HomingTargetComponent` (`Character.CapsuleComponent` (cast `/Game/Blueprints/BP_Player` (`GameplayStatics.GetPlayerPawn` 0) :!pure true)) (`self.ProjectileMovement`)))

(event `self.BoxCollision.OnComponentBeginOverlap`
  (params (OverlappedComponent :type "PrimitiveComponent Object Reference") (OtherActor :type "Actor Object Reference") (OtherComp :type "PrimitiveComponent Object Reference") (OtherBodyIndex :type Integer) (bFromSweep :type Boolean) (SweepResult :type "HitResult Structure (by ref)"))
  ;[1 1 1] Deal damage to player on impact
  (bind _asbp_player (cast `/Game/Blueprints/BP_Player` OtherActor)
    (:`then`
      (`/Game/Blueprints/BP_Player.TakeDamage` _asbp_player (`self.DamageOnImpact`)))
    (:`CastFailed`
      (cast `/Game/Blueprints/Enemies/BP_Enemy1` OtherActor
        (:`CastFailed`
          (`self.K2_DestroyActor`))))))

(event `TakeDamage`
  (params (Dmg :type "Float (double-precision)"))
  ;[1 1 1] TakeDamage
  (bind _output_get (set `self.Health` (- (`self.Health`) Dmg))))

(event `DestroyEnemy`
  (`self.K2_DestroyActor`))

(fn `UserConstructionScript`)
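; Enemy turret that turns toward the player, fires bullets, and awards points to the player when destroyed.
; Each PawnSensing sighting calls SpawnBullet, which spawns BP_Bullet at BulletSpawn after a short retriggerable delay, and interpolates Tower pitch/yaw and actor yaw toward the player.
; Entering the sphere collider snaps the actor to face the player.
; TakeDamage reduces Health, then adds PointValue to player score and destroys the turret at zero.
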(event `self.PawnSensing.OnSeePawn`
  (params (Pawn :type "Pawn Object Reference"))
  ;[1 1 1] Rotate Turret
  (bind _asbp_player (cast `/Game/Blueprints/BP_Player` Pawn))
  (`self.SpawnBullet`)
  (bind (_returnvalue_roll _returnvalue_pitch _returnvalue_yaw) (`KismetMathLibrary.BreakRotator` (`KismetMathLibrary.RInterpTo` (`self.K2_GetActorRotation`) (`KismetMathLibrary.FindLookAtRotation` (`self.K2_GetActorLocation`) (`self.K2_GetActorLocation` _asbp_player)) (`GameplayStatics.GetWorldDeltaSeconds`) (* 20.0 50.0))))
  (`SceneComponent.K2_SetWorldRotation` (`self.Tower`) (`KismetMathLibrary.MakeRotator` 0.0 _returnvalue_pitch _returnvalue_yaw) false false)
  (`self.K2_SetActorRotation` (`KismetMathLibrary.MakeRotator` 0.0 0.0 _returnvalue_yaw)))

(event `SpawnBullet`
  ;[1 1 1] SpawnBullet
  (`KismetSystemLibrary.RetriggerableDelay` 0.2)
  (`|SpawnActorFromClass` "/Game/Blueprints/Enemies/BP_Bullet.BP_Bullet_C" (`SceneComponent.K2_GetComponentToWorld` (`self.BulletSpawn`)) "Undefined" "MultiplyWithRoot" null null))

(event `TakeDamage`
  (params (Dmg :type "Float (double-precision)"))
  ;[1 1 1] TakeDamage
  (bind _output_get (set `self.Health` (- (`self.Health`) Dmg)))
  (if (<= _output_get 0.0)
    (bind _asbp_player (cast `/Game/Blueprints/BP_Player` (`GameplayStatics.GetPlayerPawn` 0)))
    (`/Game/Blueprints/BP_Player.IncreaseScore` _asbp_player (`self.PointValue`))
    (`self.K2_DestroyActor`)))

(event `self.SphereCollider.OnComponentBeginOverlap`
  (params (OverlappedComponent :type "PrimitiveComponent Object Reference") (OtherActor :type "Actor Object Reference") (OtherComp :type "PrimitiveComponent Object Reference") (OtherBodyIndex :type Integer) (bFromSweep :type Boolean) (SweepResult :type "HitResult Structure (by ref)"))
  ;[1 1 1] Initial Rotation
  (bind _asbp_player (cast `/Game/Blueprints/BP_Player` OtherActor))
  (bind (_returnvalue_roll _returnvalue_pitch _returnvalue_yaw) (`KismetMathLibrary.BreakRotator` (`KismetMathLibrary.FindLookAtRotation` (`self.K2_GetActorLocation`) (`self.K2_GetActorLocation` _asbp_player))))
  (`self.K2_SetActorRotation` (`KismetMathLibrary.MakeRotator` 0.0 _returnvalue_pitch _returnvalue_yaw)))

(fn `UserConstructionScript`)
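; BP_LootBox is a breakable loot box actor that drops a pickup and rewards the player when its LootDropper event fires.
; SpawnLoot plays a break sound and randomly spawns either a damage boost or a health pickup at the box's transform, at roughly even odds.
; LootDropper then raises the player's score multiplier and destroys the box; the box collision overlap event is empty.
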(event `self.BoxCollision.OnComponentBeginOverlap`
  (params (OverlappedComponent :type "PrimitiveComponent Object Reference") (OtherActor :type "Actor Object Reference") (OtherComp :type "PrimitiveComponent Object Reference") (OtherBodyIndex :type Integer) (bFromSweep :type Boolean) (SweepResult :type "HitResult Structure (by ref)"))
  ;[1 1 1] Spawns loot and destroys box
)

(event `LootDropper`
  ;[1 1 1] Spawns loot and destroys box
  (`self.SpawnLoot`)
  (bind _asbp_player (cast `/Game/Blueprints/BP_Player` (`GameplayStatics.GetPlayerPawn` 0)))
  (`/Game/Blueprints/BP_Player.IncreaseScoreMultiplier` _asbp_player (`self.ScoreIncValue`))
  (`self.K2_DestroyActor`))

(event `SpawnLoot`
  (bind _returnvalue (`self.GetTransform`))
  ;[1 1 1] SpawnLoot
  (`GameplayStatics.PlaySound2D` "/Game/Sounds/Lootbox_break.Lootbox_break" 1.0 1.0 0.0 null null)
  (if (< (`KismetMathLibrary.RandomIntegerInRange` 1 50) 25)
    (`|SpawnActorFromClass` "/Game/Blueprints/LootBoxBlueprints/BP_DamageBoostPickup.BP_DamageBoostPickup_C" _returnvalue "AlwaysSpawn" "MultiplyWithRoot" null null)
    (else
      (`|SpawnActorFromClass` "/Game/Blueprints/LootBoxBlueprints/BP_HealthPickup.BP_HealthPickup_C" _returnvalue "AlwaysSpawn" "MultiplyWithRoot" null null))))

(fn `UserConstructionScript`)
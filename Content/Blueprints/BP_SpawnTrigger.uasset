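; BP_SpawnTrigger is a trigger volume that spawns enemies when an actor tagged Player overlaps its box collision.
; The overlap calls SpawnEnemies, which walks the SpawnPoints array and spawns the same-index class from EnemiesToSpawn at each point's transform, regardless of collision.
; DestroyActor sits inside the loop body, so the trigger calls its own destruction after each spawn rather than once the loop completes.
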(event `self.BoxCollision.OnComponentBeginOverlap`
  (params (OverlappedComponent :type "PrimitiveComponent Object Reference") (OtherActor :type "Actor Object Reference") (OtherComp :type "PrimitiveComponent Object Reference") (OtherBodyIndex :type Integer) (bFromSweep :type Boolean) (SweepResult :type "HitResult Structure (by ref)"))
  ;[1 1 1] Detects collision with player
  (if (`self.ActorHasTag` OtherActor "Player")
    (`self.SpawnEnemies`)))

(event `SpawnEnemies`
  ;[1 1 1] Spawns enemies at each point in SpawnPoints
  (for (_array_element _array_index) (`self.SpawnPoints`)
    (`|SpawnActorFromClass` (`|GetArrayItem` (`self.EnemiesToSpawn`) _array_index) (`self.GetTransform` _array_element) "AlwaysSpawn" "MultiplyWithRoot" null null)
    (`self.K2_DestroyActor`)))

(fn `UserConstructionScript`)